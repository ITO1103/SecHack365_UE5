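; Player-flown jet for the USB level, with input held for three seconds at start and hits flagging USBClash on SH365GameInstance unless USBSuccess is set.
; Axis inputs adjust clamped thrust and apply interpolated local yaw, pitch and roll.
; Tick moves it forward with sweep, easing speed increases by Drag and fading in gravity below MinThrustToNotFall.
; It also records altitude and writes a movement-derived speed readout to the game instance.
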(event OnComponentHit(StaticMesh)
  (params (HitComponent :type Primitive%20Component%20Object%20Reference) (OtherActor :type Actor%20Object%20Reference) (OtherComp :type Primitive%20Component%20Object%20Reference) (NormalImpulse :type Vector :default "0, 0, 0") (Hit :type Hit%20Result%20Structure%20%28by%20ref%29))
  (bind _assh365game_instance (Utilities|Casting|CastToSH365GameInstance (Game|GetGameInstance)))
  (if (not (Variables|/Game/SH365GameInstance.SH365GameInstance_C|GetUSBSuccess _assh365game_instance))
    (Variables|/Game/SH365GameInstance.SH365GameInstance_C|SetUSBClash _assh365game_instance true)
    (Development|PrintString "Hello")))

(event EventBeginPlay
  (bind _returnvalue (Game|Player|GetPlayerPawn 0))
  (bind _output_get (Variables|Default|SetThrustSpeed (Variables|Default|GetMinThrustToNotFall)))
  (Variables|Default|SetCurrentSpeed _output_get)
  ;[1 1 1] Disable input
  (Input|DisableInput _returnvalue 0)
  (Utilities|FlowControl|Delay 3.0)
  (Input|EnableInput _returnvalue 0))

(event Collision|EventActorBeginOverlap
  (params (OtherActor :type Actor%20Object%20Reference)))

(event EventTick
  (params (DeltaSeconds :type Float%20%28single-precision%29))
  (CallFunction|UpdatePosition DeltaSeconds)
  (CallFunction|PrintVali)
  (Variables|Default|SetAltitude (Math|Float|Truncate (.z (Transformation|GetActorLocation))))
  ;[1 1 1] AirSpeed
  (CallFunction|CalSpeed)
  (Variables|Default|SetPreviousLocation (Transformation|GetActorLocation)))

(event Input|AxisEvents|InputAxisThrust
  (params (AxisValue :type Float%20%28single-precision%29))
  (Variables|Default|SetThrustSpeed (Math|Float|Clamp(Float) (+ (* AxisValue (Utilities|Time|GetWorldDeltaSeconds) (Variables|Default|GetThrustMultiplier)) (Variables|Default|GetThrustSpeed)) 0.0 (Variables|Default|GetMaxThrustSpeed))))

(event Input|AxisEvents|InputAxisYaw
  (params (AxisValue :type Float%20%28single-precision%29))
  (CallFunction|UpdateYaw (Utilities|Time|GetWorldDeltaSeconds) AxisValue))

(event Input|AxisEvents|InputAxisPitch
  (params (AxisValue :type Float%20%28single-precision%29))
  (CallFunction|UpdatePitch (Utilities|Time|GetWorldDeltaSeconds) AxisValue))

(event Input|AxisEvents|InputAxisRoll
  (params (AxisValue :type Float%20%28single-precision%29))
  (CallFunction|UpdateRoll (Utilities|Time|GetWorldDeltaSeconds) AxisValue))

(event Input|KeyboardEvents|8
  (params (Key :type Key%20Structure :default "None"))
  (:Pressed
    (Game|SpawnActorfromClass "BP_JET_C" (Math|Transform|MakeTransform (Transformation|GetActorLocation) (Transformation|GetActorRotation) "1.000000,1.000000,1.000000") "Undefined" "MultiplyWithRoot" 0 0)))

(fn ConstructionScript)

(fn UpdatePosition
  (params (DeltaSeconds :type Float%20%28double-precision%29))
  (Variables|Default|SetCurrentSpeed (Math|Float|SelectFloat (Variables|Default|GetThrustSpeed) (Math|Interpolation|FInterpTo (Variables|Default|GetCurrentSpeed) (Variables|Default|GetThrustSpeed) DeltaSeconds (Variables|Default|GetDrag)) (< (Variables|Default|GetThrustSpeed) (Variables|Default|GetCurrentSpeed))))
  (LocalVariables|SetNewPosition (* (* (Variables|Default|GetCurrentSpeed) DeltaSeconds) (Transformation|GetActorForwardVector)))
  (Variables|Default|SetAppliedGravity (Math|Float|MapRangeClamped (Variables|Default|GetCurrentSpeed) 0.0 (Variables|Default|GetMinThrustToNotFall) (Variables|Default|GetGravity) 0.0))
  (Transformation|AddActorWorldOffset (Math|Vector|MakeVector (.X (Math|Vector|BreakVector (LocalVariables|GetNewPosition))) (.Y (Math|Vector|BreakVector (LocalVariables|GetNewPosition))) (- (.Z (Math|Vector|BreakVector (LocalVariables|GetNewPosition))) (* (Variables|Default|GetAppliedGravity) DeltaSeconds))) true))

(fn UpdateYaw
  (params (DeltaSeconds :type Float%20%28double-precision%29) (Yaw :type Float%20%28double-precision%29))
  (Variables|Default|SetTargetYaw Yaw)
  (bind _output_get (Variables|Default|SetCurrentYaw (Math|Interpolation|FInterpTo (Variables|Default|GetCurrentYaw) (Variables|Default|GetTargetYaw) DeltaSeconds 1e+01)))
  (Transformation|AddActorLocalRotation (Math|Rotator|MakeRotator 0.0 0.0 (* _output_get DeltaSeconds 1e+02)) false false))

(fn UpdatePitch
  (params (DeltaSeconds :type Float%20%28double-precision%29) (Pitch :type Float%20%28double-precision%29))
  (Variables|Default|SetTargetPitch Pitch)
  (bind _output_get (Variables|Default|SetCurrentPitch (Math|Interpolation|FInterpTo (Variables|Default|GetCurrentPitch) (Variables|Default|GetTargetPitch) DeltaSeconds 1e+01)))
  (Transformation|AddActorLocalRotation (Math|Rotator|MakeRotator 0.0 (* _output_get DeltaSeconds 1e+02) 0.0) false false))

(fn UpdateRoll
  (params (DeltaSeconds :type Float%20%28double-precision%29) (Roll :type Float%20%28double-precision%29))
  (Variables|Default|SetTargetRoll Roll)
  (bind _output_get (Variables|Default|SetCurrentRoll (Math|Interpolation|FInterpTo (Variables|Default|GetCurrentRoll) (Variables|Default|GetTargetRoll) DeltaSeconds 1e+01)))
  (Transformation|AddActorLocalRotation (Math|Rotator|MakeRotator (* _output_get DeltaSeconds 1e+02) 0.0 0.0) false false))

(fn PrintVali)

(fn CalSpeed
  (bind _returnvalue (Transformation|GetActorLocation))
  (bind _previouslocation (Variables|Default|GetPreviousLocation))
  (bind _returnvalue_2 (- _previouslocation _returnvalue))
  (bind _assh365game_instance (Utilities|Casting|CastToSH365GameInstance (Game|GetGameInstance)))
  (Variables|/Game/SH365GameInstance.SH365GameInstance_C|SetINS_USBSpeed _assh365game_instance (Math|Float|Truncate (/ (/ (/ (+ (/ (Math|Float|Power (.x _returnvalue_2) 2.0) 2.0) (/ (Math|Float|Power (.y _returnvalue_2) 2.0) 2.0) (/ (Math|Float|Power (.z _returnvalue_2) 2.0) 2.0)) 3.0) (Utilities|Time|GetWorldDeltaSeconds)) 1e+01))))