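; Sets up the USB stage, where clues describe a USB stick and the computer it is about to be plugged into.
; On BeginPlay it adds caption, HUD and escape widgets, plays a quiet circuit sound and resets the clue index in SH365GameInstance.
; USBLevel (1 or 2) selects the Japanese clue texts stored there and the fixed spots where Infomation actors spawn.
; Tick is empty, and the speed/location debug code is disconnected.
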(event EventBeginPlay
  (bind _returnvalue (UserInterface|CreateWidget "/Game/Level/2_USB/WBP_2_caption.WBP_2_caption_C"))
  (bind _returnvalue_2 (UserInterface|CreateWidget "/Game/Level/2_USB/2_HUD.2_HUD_C"))
  (UserInterface|Viewport|AddtoViewport _returnvalue 0)
  (bind _returnvalue_3 (UserInterface|CreateWidget "/Game/Level/WB_Escape.WB_Escape_C"))
  (UserInterface|Viewport|AddtoViewport _returnvalue_3 2)
  (Audio|PlaySound2D "/Game/BGM/Mechanical_Circuit.Mechanical_Circuit" 0.1 1.0 0.0 0 0)
  (bind _assh365game_instance (Utilities|Casting|CastToSH365GameInstance (Game|GetGameInstance)))
  (Variables|/Game/SH365GameInstance.SH365GameInstance_C|SetUSBinfoindex _assh365game_instance 0)
  (Variables|/Game/SH365GameInstance.SH365GameInstance_C|SetUSBinfo _assh365game_instance (Utilities|Array|MakeArray "" "" "" ""))
  (switch int (Variables|/Game/SH365GameInstance.SH365GameInstance_C|GetUSBLevel _assh365game_instance)
    (:1
      (Variables|/Game/SH365GameInstance.SH365GameInstance_C|SetUSBinfo _assh365game_instance (Utilities|Array|MakeArray "" "いつも家で使っているUSBに似ている" "これから挿すのは会社のパソコン" "会社のポリシーでは許可されてないデバイスは挿してはいけないんだっけ...？"))
      (Game|SpawnActorfromClass "/Game/Level/2_USB/Infomation.Infomation_C" (Math|Transform|MakeTransform "10140.000000,-19080.000000,1770.000000" "0, 0, 0" "1.000000,1.000000,1.000000") "Undefined" "MultiplyWithRoot" 0 0)
      (Game|SpawnActorfromClass "/Game/Level/2_USB/Infomation.Infomation_C" (Math|Transform|MakeTransform "22140.000000,-8480.000000,10000.000000" "0, 0, 0" "1.000000,1.000000,1.000000") "Undefined" "MultiplyWithRoot" 0 0)
      (Game|SpawnActorfromClass "/Game/Level/2_USB/Infomation.Infomation_C" (Math|Transform|MakeTransform "10250.000000,20930.000000,1444.000000" "0, 0, 0" "1.000000,1.000000,1.000000") "Undefined" "MultiplyWithRoot" 0 0))
    (:2
      (Variables|/Game/SH365GameInstance.SH365GameInstance_C|SetUSBinfo _assh365game_instance (Utilities|Array|MakeArray "表面に少し傷があり、使用感がある" "ラベルには「卒論データ」と書かれている" "これから挿すのは個人のパソコン" "通勤途中の道で拾った"))
      (Game|SpawnActorfromClass "/Game/Level/2_USB/Infomation.Infomation_C" (Math|Transform|MakeTransform "23000.000000,-19080.000000,26000.000000" "0, 0, 0" "1.000000,1.000000,1.000000") "Undefined" "MultiplyWithRoot" 0 0)
      (Game|SpawnActorfromClass "/Game/Level/2_USB/Infomation.Infomation_C" (Math|Transform|MakeTransform "26000.000000,6000.000000,5000.000000" "0, 0, 0" "1.000000,1.000000,1.000000") "Undefined" "MultiplyWithRoot" 0 0)
      (Game|SpawnActorfromClass "/Game/Level/2_USB/Infomation.Infomation_C" (Math|Transform|MakeTransform "-3000.000000,20930.000000,1444.000000" "0, 0, 0" "1.000000,1.000000,1.000000") "Undefined" "MultiplyWithRoot" 0 0)
      (Game|SpawnActorfromClass "/Game/Level/2_USB/Infomation.Infomation_C" (Math|Transform|MakeTransform "26000.000000,20930.000000,1444.000000" "0, 0, 0" "1.000000,1.000000,1.000000") "Undefined" "MultiplyWithRoot" 0 0))))

(event Collision|EventActorBeginOverlap
  (params (OtherActor :type Actor%20Object%20Reference)))

(event EventTick
  (params (DeltaSeconds :type Float%20%28single-precision%29)))

(fn ConstructionScript)