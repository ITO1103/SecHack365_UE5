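; Quiz level actor that runs one quiz round and shows its result, exploding when the player answers wrong.
; BeginPlay resets GameInstance quiz flags, adds the escape and quiz widgets, and loads a random DT_Quiz row into the GameInstance.
; Tick polls those flags once: timeout or a correct answer opens the result widget directly.
; A wrong answer spawns an explosion with sound, sets WeakFlag, then shows the result after a short delay.
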(event EventBeginPlay
  (CallFunction|Init)
  (bind _returnvalue (UserInterface|CreateWidget "/Game/Level/WB_Escape.WB_Escape_C"))
  (UserInterface|Viewport|AddtoViewport _returnvalue 2)
  (bind _returnvalue_2 (UserInterface|CreateWidget "/Game/Level/3_Quiz/3_WBP_inQuiz.3_WBP_inQuiz_C"))
  (UserInterface|Viewport|AddtoViewport _returnvalue_2 1)
  (Variables|/Script/Engine.PlayerController|SetbShowMouseCursor (Game|GetPlayerController 0) true)
  (bind _assh365game_instance (Utilities|Casting|CastToSH365GameInstance (Game|GetGameInstance)))
  (Development|PrintString (Utilities|String|ToString(Integer) (Variables|/Game/SH365GameInstance.SH365GameInstance_C|GetINS_Quizindex _assh365game_instance)) true true "(R=1.000000,G=1.000000,B=1.000000,A=1.000000)")
  (CallFunction|QuizDT))

(event EventTick
  (params (DeltaSeconds :type Float%20%28single-precision%29))
  (bind _assh365game_instance (Utilities|Casting|CastToSH365GameInstance (Game|GetGameInstance)))
  ;[1 1 1] タイムアップだったら爆発しない
  (if (Variables|/Game/SH365GameInstance.SH365GameInstance_C|GetINS_TimeUP _assh365game_instance)
    (Utilities|FlowControl|DoOnce false
      (:Completed
        ;[1 1 1] リザルト画面表示
        (bind _returnvalue (UserInterface|CreateWidget "/Game/Level/3_Quiz/3_WBP_Result.3_WBP_Result_C" :!label _label))
        (UserInterface|Viewport|AddtoViewport _returnvalue 1)))
    (else
      ;[1 1 1] ボタンが押されたのを検出 + 脆弱でだったら→一度だけ実行
      (if (Variables|/Game/SH365GameInstance.SH365GameInstance_C|GetINS_QuizButtonPressed _assh365game_instance)
        (Utilities|FlowControl|DoOnce false
          (:Completed
            ;[1 1 1] 間違っていたら爆発
            (if (Variables|/Game/SH365GameInstance.SH365GameInstance_C|GetINS_QuizResault _assh365game_instance)
              (goto _label)
              (else
                ;[1 1 1] 爆発部分
                (Effects|SpawnEmitteratLocation "/Game/StarterContent/Particles/P_Explosion.P_Explosion" (Transformation|GetActorLocation) "0.000000,0.000000,11.000000" "11.000000,11.000000,11.000000")
                (Audio|PlaySound2D "/Game/StarterContent/Audio/Explosion01.Explosion01" 1.0 1.0 0.0 0 0)
                (Variables|/Game/SH365GameInstance.SH365GameInstance_C|SetWeakFlag _assh365game_instance true)
                ;[1 1 1] 爆発の余韻1秒
                (Utilities|FlowControl|Delay 1.0)
                (goto _label)))))))))

(fn ConstructionScript)

(fn QuizDT
  (bind _outrownames (DataTable|GetDataTableRowNames "/Game/Level/3_Quiz/CSV/DT_Quiz.DT_Quiz"))
  (bind _returnvalue (Utilities|GetDataTableRow "/Game/Level/3_Quiz/CSV/DT_Quiz.DT_Quiz" (.OutItem (Utilities|Array|Random _outrownames)))
    (:then
      (bind _assh365game_instance (Utilities|Casting|CastToSH365GameInstance (Game|GetGameInstance)))
      (Variables|/Game/SH365GameInstance.SH365GameInstance_C|SetINS_Quiztext _assh365game_instance (.Quiz (Utilities|Struct|BreakST_Quiz _returnvalue)))
      (Variables|/Game/SH365GameInstance.SH365GameInstance_C|SetINS_QuizCorrect _assh365game_instance (.Correct (Utilities|Struct|BreakST_Quiz _returnvalue)))
      (Variables|/Game/SH365GameInstance.SH365GameInstance_C|SetINS_QuizReason _assh365game_instance (.Reason (Utilities|Struct|BreakST_Quiz _returnvalue))))))

(fn Init
  (bind _assh365game_instance (Utilities|Casting|CastToSH365GameInstance (Game|GetGameInstance)))
  (Variables|/Game/SH365GameInstance.SH365GameInstance_C|SetINS_QuizButtonPressed _assh365game_instance false)
  (Variables|/Game/SH365GameInstance.SH365GameInstance_C|SetINS_QuizResault _assh365game_instance false)
  (Variables|/Game/SH365GameInstance.SH365GameInstance_C|SetINS_TimeUP _assh365game_instance false))