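; Login-level actor for a password-security game that explodes when the player's submitted password is weak, then shows the tips widget.
; BeginPlay resets GameInstance state and builds the UI; Tick polls it for timeout (no explosion) or button press.
; WeakJudgmentFunction combines length, ID-match, DataTable, C++ regex and zxcvbn checks into level-specific verdicts, including reuse of saved passwords.
; SQL injection payload matches quit the game.
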(event EventBeginPlay
  ;[1 1 1] 最終レベルのみ
  (bind _assh365game_instance (Utilities|Casting|CastToSH365GameInstance (Game|GetGameInstance)))
  (if (Variables|/Game/SH365GameInstance.SH365GameInstance_C|GetINS_PWLastLevel _assh365game_instance)
    (bind _returnvalue (UserInterface|CreateWidget "/Game/Level/1_Login/WBP_Final.WBP_Final_C"))
    (UserInterface|Viewport|AddtoViewport _returnvalue 3))
  (CallFunction|InitializeValialances)
  (bind _returnvalue_2 (UserInterface|CreateWidget "/Game/Level/WB_Escape.WB_Escape_C"))
  (UserInterface|Viewport|AddtoViewport _returnvalue_2 2)
  (bind _returnvalue_3 (UserInterface|CreateWidget "/Game/Level/1_Login/WBP_1_Regulation.WBP_1_Regulation_C"))
  (UserInterface|Viewport|AddtoViewport _returnvalue_3 1)
  (bind _returnvalue_4 (UserInterface|CreateWidget "/Game/Level/1_Login/WBP_Login.WBP_Login_C"))
  (UserInterface|Viewport|AddtoViewport _returnvalue_4 0)
  (Variables|/Script/Engine.PlayerController|SetbShowMouseCursor (Game|GetPlayerController 0) true)
  (bind _assh365game_instance_2 (Utilities|Casting|CastToSH365GameInstance (Game|GetGameInstance)))
  (Development|PrintString (Utilities|String|ToString(Integer) (Variables|/Game/SH365GameInstance.SH365GameInstance_C|GetIDPWLevel _assh365game_instance_2)) true true "(R=1.000000,G=1.000000,B=1.000000,A=1.000000)"))

(event EventTick
  (params (DeltaSeconds :type Float%20%28single-precision%29))
  (bind _assh365game_instance (Utilities|Casting|CastToSH365GameInstance (Game|GetGameInstance)))
  ;[1 1 1] タイムアップだったら爆発しない
  (if (Variables|/Game/SH365GameInstance.SH365GameInstance_C|GetINS_TimeUP _assh365game_instance)
    (Utilities|FlowControl|DoOnce false
      (:Completed
        ;[1 1 1] リザルト画面表示
        (bind _returnvalue (UserInterface|CreateWidget "/Game/Level/1_Login/WBP_LoginTips.WBP_LoginTips_C" :!label _label))
        (UserInterface|Viewport|AddtoViewport _returnvalue 1)))
    (else
      ;[1 1 1] ボタンが押されたのを検出 + 脆弱でだったら→一度だけ実行
      (if (Variables|/Game/SH365GameInstance.SH365GameInstance_C|GetINS_1_ButtonPress _assh365game_instance)
        (bind _returnvalue_2 (Actor|GetActorOfClass "/Script/SecHack.RegexPW"))
        (if (Variables|/Script/SecHack.RegexPW|GetSameWithGenericErrorBasedPayloadsFlag _returnvalue_2)
          (Game|QuitGame 0 "Quit" false)
          (else
            (Utilities|FlowControl|DoOnce false
              (:Completed
                (CallFunction|WeakJudgmentFunction)
                ;[1 1 1] 脆弱→爆発
                (if (Variables|/Game/SH365GameInstance.SH365GameInstance_C|GetWeakFlag _assh365game_instance)
                  ;[1 1 1] 爆発部分
                  (Effects|SpawnEmitteratLocation "/Game/StarterContent/Particles/P_Explosion.P_Explosion" (Transformation|GetActorLocation) "0.000000,0.000000,11.000000" "11.000000,11.000000,11.000000")
                  (Audio|PlaySound2D "/Game/StarterContent/Audio/Explosion01.Explosion01" 1.0 1.0 0.0 0 0)
                  (Variables|/Game/SH365GameInstance.SH365GameInstance_C|SetWeakFlag _assh365game_instance true)
                  ;[1 1 1] 爆発の余韻1秒
                  (Utilities|FlowControl|Delay 1.0)
                  (goto _label)
                  (else
                    (goto _label)))))))))))

(fn ConstructionScript)

(fn InitializeValialances
  ;[1 1 1] GameInstanceの変数初期化
  (bind _assh365game_instance (Utilities|Casting|CastToSH365GameInstance (Game|GetGameInstance)))
  (Variables|/Game/SH365GameInstance.SH365GameInstance_C|SetINS_ID==PW _assh365game_instance false)
  (Variables|/Game/SH365GameInstance.SH365GameInstance_C|SetINS_IDweek _assh365game_instance false)
  (Variables|/Game/SH365GameInstance.SH365GameInstance_C|SetINS_PWweek _assh365game_instance false)
  (Variables|/Game/SH365GameInstance.SH365GameInstance_C|SetINS_RegButton _assh365game_instance false)
  (Variables|/Game/SH365GameInstance.SH365GameInstance_C|SetINS_TimeUP _assh365game_instance false)
  (Variables|/Game/SH365GameInstance.SH365GameInstance_C|SetINS_IDPWweek _assh365game_instance false)
  (Variables|/Game/SH365GameInstance.SH365GameInstance_C|SetINS_1_ButtonPress _assh365game_instance false)
  (Variables|/Game/SH365GameInstance.SH365GameInstance_C|SetWeakFlag _assh365game_instance false)
  (Variables|/Game/SH365GameInstance.SH365GameInstance_C|SetINS_WeekScore _assh365game_instance 0.0)
  (Variables|/Game/SH365GameInstance.SH365GameInstance_C|SetINS_PWStr _assh365game_instance "")
  (Variables|/Game/SH365GameInstance.SH365GameInstance_C|SetINS_IDStr _assh365game_instance "")
  (Variables|Default|SetSQLi false)
  (Variables|Default|Set500-worst-passwords false))

(fn SaveLevelPW
  ;[1 1 1] Level1~5のPWを保存
  (bind _assh365game_instance (Utilities|Casting|CastToSH365GameInstance (Game|GetGameInstance)))
  (switch int (Variables|/Game/SH365GameInstance.SH365GameInstance_C|GetIDPWLevel _assh365game_instance)
    (:1
      (Variables|/Game/SH365GameInstance.SH365GameInstance_C|SetLevel1PW _assh365game_instance (Utilities|String|ToString(Text) (Variables|/Game/SH365GameInstance.SH365GameInstance_C|GetINS_PWStr _assh365game_instance))))
    (:2
      (Variables|/Game/SH365GameInstance.SH365GameInstance_C|SetLevel2PW _assh365game_instance (Utilities|String|ToString(Text) (Variables|/Game/SH365GameInstance.SH365GameInstance_C|GetINS_PWStr _assh365game_instance))))
    (:3
      (Variables|/Game/SH365GameInstance.SH365GameInstance_C|SetLevel3PW _assh365game_instance (Utilities|String|ToString(Text) (Variables|/Game/SH365GameInstance.SH365GameInstance_C|GetINS_PWStr _assh365game_instance))))
    (:4
      (Variables|/Game/SH365GameInstance.SH365GameInstance_C|SetLevel4PW _assh365game_instance (Utilities|String|ToString(Text) (Variables|/Game/SH365GameInstance.SH365GameInstance_C|GetINS_PWStr _assh365game_instance))))
    (:5
      (Variables|/Game/SH365GameInstance.SH365GameInstance_C|SetLevel5PW _assh365game_instance (Utilities|String|ToString(Text) (Variables|/Game/SH365GameInstance.SH365GameInstance_C|GetINS_PWStr _assh365game_instance))))))

(fn IDLenFunction
  ;[1 1 1] IDの文字列の長さの判定
  (bind _assh365game_instance (Utilities|Casting|CastToSH365GameInstance (Game|GetGameInstance)))
  ;;[1 1 1] IDの長さ取得
  (bind _output_get (Variables|/Game/SH365GameInstance.SH365GameInstance_C|SetINS_IDLen _assh365game_instance (Utilities|String|Len (Utilities|String|ToString(Text) (Variables|/Game/SH365GameInstance.SH365GameInstance_C|GetINS_IDStr _assh365game_instance)))))
  ;;[1 1 1] IDが10文字以下か判定
  (if (> _output_get 9)
    (Development|PrintString (Utilities|String|ToString(Integer) _output_get))
    (Variables|/Game/SH365GameInstance.SH365GameInstance_C|SetINS_IDweek _assh365game_instance false)
    (else
      (Development|PrintString (Utilities|String|ToString(Integer) _output_get))
      (Variables|/Game/SH365GameInstance.SH365GameInstance_C|SetINS_IDweek _assh365game_instance true))))

(fn PWLenFunction
  ;[1 1 1] PWの文字列の長さの判定
  (bind _assh365game_instance (Utilities|Casting|CastToSH365GameInstance (Game|GetGameInstance)))
  ;;[1 1 1] IDの長さ取得
  (bind _output_get (Variables|/Game/SH365GameInstance.SH365GameInstance_C|SetINS_PWLen _assh365game_instance (Utilities|String|Len (Utilities|String|ToString(Text) (Variables|/Game/SH365GameInstance.SH365GameInstance_C|GetINS_PWStr _assh365game_instance)))))
  ;;[1 1 1] IDが10文字以下か判定
  (if (> _output_get 9)
    (Development|PrintString (Utilities|String|ToString(Integer) _output_get))
    (Variables|/Game/SH365GameInstance.SH365GameInstance_C|SetINS_PWweek _assh365game_instance false)
    (else
      (Development|PrintString (Utilities|String|ToString(Integer) _output_get))
      (Variables|/Game/SH365GameInstance.SH365GameInstance_C|SetINS_PWweek _assh365game_instance true))))

(fn ID==PWFunction
  (bind _assh365game_instance (Utilities|Casting|CastToSH365GameInstance (Game|GetGameInstance)))
  (if (Utilities|Enum|Equal(Enum) (Utilities|String|ToString(Text) (Variables|/Game/SH365GameInstance.SH365GameInstance_C|GetINS_IDStr _assh365game_instance)) (Utilities|String|ToString(Text) (Variables|/Game/SH365GameInstance.SH365GameInstance_C|GetINS_PWStr _assh365game_instance)))
    (Development|PrintString "ID==PW!!")
    (Variables|/Game/SH365GameInstance.SH365GameInstance_C|SetINS_ID==PW _assh365game_instance true)
    (else
      (Development|PrintString "ID!=PW"))))

(fn WeakScoreCalculator
  (bind _returnvalue (Actor|GetActorOfClass "/Script/SecHack.CheckPW"))
  (bind _assh365game_instance (Utilities|Casting|CastToSH365GameInstance (Game|GetGameInstance)))
  (bind _output_get (Variables|/Game/SH365GameInstance.SH365GameInstance_C|SetINS_WeekScore _assh365game_instance (/ (Math|Conversions|ToFloat(Integer) (Math|Float|Truncate (* (Variables|/Script/SecHack.CheckPW|GetPasswordEntropy _returnvalue) 1e+03))) 1e+03)))
  (Development|PrintString (Utilities|String|ToString(Float) _output_get)))

(fn WeakJudgmentFunction
  (bind _assh365game_instance (Utilities|Casting|CastToSH365GameInstance (Game|GetGameInstance)))
  (CallFunction|IDLenFunction)
  (CallFunction|PWLenFunction)
  (CallFunction|SaveLevelPW)
  (CallFunction|ID==PWFunction)
  (CallFunction|CheckWeakPW)
  (CallFunction|CheckSQLi)
  ;[1 1 1] C++
  (bind _outactors (Actor|GetAllActorsOfClass "/Script/SecHack.RegexPW"))
  (Class|RegexPW|SamewithGenericErrorBasedPayloads _outactors (Utilities|String|ToString(Text) (Variables|/Game/SH365GameInstance.SH365GameInstance_C|GetINS_PWStr _assh365game_instance)))
  (Class|RegexPW|SamewithWeakPassword _outactors (Utilities|String|ToString(Text) (Variables|/Game/SH365GameInstance.SH365GameInstance_C|GetINS_PWStr _assh365game_instance)))
  (Class|RegexPW|RegexFunction _outactors (Utilities|String|ToString(Text) (Variables|/Game/SH365GameInstance.SH365GameInstance_C|GetINS_PWStr _assh365game_instance)))
  (Class|RegexPW|NoRegexFlags _outactors (Utilities|String|ToString(Text) (Variables|/Game/SH365GameInstance.SH365GameInstance_C|GetINS_PWStr _assh365game_instance)))
  (bind _returnvalue (Actor|GetActorOfClass "/Script/SecHack.RegexPW"))
  (bind _returnvalue_2 (Actor|GetActorOfClass "/Script/SecHack.CheckPW"))
  (Class|CheckPW|RunPasswordChecks _returnvalue_2 (Utilities|Array|MakeArray "" (Utilities|String|ToString(Text) (Variables|/Game/SH365GameInstance.SH365GameInstance_C|GetINS_PWStr _assh365game_instance))))
  ;[1 1 1] C++実行後でないといけない奴ら
  (bind _assh365game_instance_2 (Utilities|Casting|CastToSH365GameInstance (Game|GetGameInstance)))
  (CallFunction|WeakScoreCalculator)
  (CallFunction|ZxcvbnReason)
  (if (Variables|/Game/SH365GameInstance.SH365GameInstance_C|GetINS_SQLi _assh365game_instance_2)
    (Game|QuitGame 0 "Quit" false)
    (else
      (switch int (Variables|/Game/SH365GameInstance.SH365GameInstance_C|GetIDPWLevel _assh365game_instance)
        (:1
          ;[1 1 1] Level1
          (Utilities|FlowControl|Sequence
            (:then_0
              (if (Variables|/Game/SH365GameInstance.SH365GameInstance_C|GetINS_PWweek _assh365game_instance)
                (Variables|/Game/SH365GameInstance.SH365GameInstance_C|SetWeakFlag _assh365game_instance true :!label _label)
                (Variables|/Game/SH365GameInstance.SH365GameInstance_C|SetLevel1PW _assh365game_instance (Utilities|String|ToString(Text) (Variables|/Game/SH365GameInstance.SH365GameInstance_C|GetINS_PWStr _assh365game_instance)))))
            (:then_1
              (if (Variables|/Game/SH365GameInstance.SH365GameInstance_C|GetINS_ID==PW _assh365game_instance)
                (goto _label)))
            (:then_2
              (if (Variables|/Game/SH365GameInstance.SH365GameInstance_C|GetINS_500-worst-password _assh365game_instance_2)
                (goto _label)))
            (:then_3
              (if (Variables|/Script/SecHack.RegexPW|GetnoSymbolFlag _returnvalue)
                (goto _label)))
            (:then_4
              (if (Variables|/Script/SecHack.RegexPW|GetnoNumberFlag _returnvalue)
                (goto _label)))
            (:then_5
              (if (Variables|/Script/SecHack.RegexPW|GetnoUpperAlphabetFlag _returnvalue)
                (goto _label)))
            (:then_6
              (if (Variables|/Script/SecHack.RegexPW|GetnoLowerAlphabetFlag _returnvalue)
                (goto _label)))))
        (:2
          ;[1 1 1] Level2（10文字以上）
          (if (Variables|/Game/SH365GameInstance.SH365GameInstance_C|GetINS_PWweek _assh365game_instance)
            (Variables|/Game/SH365GameInstance.SH365GameInstance_C|SetWeakFlag _assh365game_instance false)
            (else
              (Utilities|FlowControl|Sequence
                (:then_0
                  (if (Variables|/Game/SH365GameInstance.SH365GameInstance_C|GetINS_500-worst-password _assh365game_instance_2)
                    (Variables|/Game/SH365GameInstance.SH365GameInstance_C|SetWeakFlag _assh365game_instance true :!label _label_2)
                    (Variables|/Game/SH365GameInstance.SH365GameInstance_C|SetLevel2PW _assh365game_instance (Utilities|String|ToString(Text) (Variables|/Game/SH365GameInstance.SH365GameInstance_C|GetINS_PWStr _assh365game_instance)))))
                (:then_1
                  (if (Variables|/Script/SecHack.RegexPW|GetnoSymbolFlag _returnvalue)
                    (goto _label_2)))
                (:then_2
                  (if (Variables|/Script/SecHack.RegexPW|GetnoNumberFlag _returnvalue)
                    (goto _label_2)))
                (:then_3
                  (if (Variables|/Script/SecHack.RegexPW|GetnoUpperAlphabetFlag _returnvalue)
                    (goto _label_2)))
                (:then_4
                  (if (Variables|/Script/SecHack.RegexPW|GetnoLowerAlphabetFlag _returnvalue)
                    (goto _label_2)))
                (:then_5
                  (if (Variables|/Game/SH365GameInstance.SH365GameInstance_C|GetINS_ID==PW _assh365game_instance)
                    (goto _label_2)))
                (:then_6
                  (if true
                    (goto _label_2)))
                (:then_7
                  (if true
                    (goto _label_2)))))))
        (:3
          ;[1 1 1] Level3（10文字以上+記号/数字を入れる）
          (if (Variables|/Game/SH365GameInstance.SH365GameInstance_C|GetINS_PWweek _assh365game_instance)
            (Variables|/Game/SH365GameInstance.SH365GameInstance_C|SetWeakFlag _assh365game_instance false :!label _label_3)
            (elif (Variables|/Script/SecHack.RegexPW|GetnoSymbolFlag _returnvalue)
              (goto _label_3)
              (elif (Variables|/Script/SecHack.RegexPW|GetnoNumberFlag _returnvalue)
                (goto _label_3)
                (else
                  (Utilities|FlowControl|Sequence
                    (:then_0
                      (if (Variables|/Game/SH365GameInstance.SH365GameInstance_C|GetINS_500-worst-password _assh365game_instance_2)
                        (Variables|/Game/SH365GameInstance.SH365GameInstance_C|SetWeakFlag _assh365game_instance true :!label _label_4)
                        (Variables|/Game/SH365GameInstance.SH365GameInstance_C|SetLevel3PW _assh365game_instance (Utilities|String|ToString(Text) (Variables|/Game/SH365GameInstance.SH365GameInstance_C|GetINS_PWStr _assh365game_instance)))))
                    (:then_1
                      (if (Variables|/Script/SecHack.RegexPW|GetnoUpperAlphabetFlag _returnvalue)
                        (goto _label_4)))
                    (:then_2
                      (if true
                        (goto _label_4)))
                    (:then_3
                      (if (Variables|/Game/SH365GameInstance.SH365GameInstance_C|GetINS_ID==PW _assh365game_instance)
                        (goto _label_4)))
                    (:then_4
                      (if true
                        (goto _label_4)))
                    (:then_5
                      (if true
                        (goto _label_4)))
                    (:then_6
                      (if true
                        (goto _label_4)))
                    (:then_7
                      (if true
                        (goto _label_4)))))))))
        (:4
          ;[1 1 1] Level4（10文字以上+記号/数字両方入れる+大/小文字 + zxcvbn<10）
          (if (Variables|/Game/SH365GameInstance.SH365GameInstance_C|GetINS_PWweek _assh365game_instance)
            (Variables|/Game/SH365GameInstance.SH365GameInstance_C|SetWeakFlag _assh365game_instance false :!label _label_5)
            (elif (Variables|/Script/SecHack.RegexPW|GetnoSymbolFlag _returnvalue)
              (goto _label_5)
              (elif (Variables|/Script/SecHack.RegexPW|GetnoNumberFlag _returnvalue)
                (goto _label_5)
                (elif (Variables|/Script/SecHack.RegexPW|GetnoUpperAlphabetFlag _returnvalue)
                  (goto _label_5)
                  (elif (Variables|/Script/SecHack.RegexPW|GetnoLowerAlphabetFlag _returnvalue)
                    (goto _label_5)
                    (elif true
                      (bind _assh365game_instance_3 (Utilities|Casting|CastToSH365GameInstance (Game|GetGameInstance)))
                      (if (> 1e+01 (Variables|/Game/SH365GameInstance.SH365GameInstance_C|GetINS_WeekScore _assh365game_instance_3))
                        (Variables|/Game/SH365GameInstance.SH365GameInstance_C|SetWeakFlag _assh365game_instance true)
                        (Variables|/Game/SH365GameInstance.SH365GameInstance_C|SetLevel4PW _assh365game_instance (Utilities|String|ToString(Text) (Variables|/Game/SH365GameInstance.SH365GameInstance_C|GetINS_PWStr _assh365game_instance)))))))))))
        (:5
          ;[1 1 1] Level5
          (if (Utilities|Enum|Equal(Enum) (Utilities|String|ToString(Text) (Variables|/Game/SH365GameInstance.SH365GameInstance_C|GetINS_PWStr _assh365game_instance)) (Variables|/Game/SH365GameInstance.SH365GameInstance_C|GetLevel1PW _assh365game_instance))
            (Variables|/Game/SH365GameInstance.SH365GameInstance_C|SetWeakFlag _assh365game_instance true :!label _label_6)
            (bind _assh365game_instance_4 (Utilities|Casting|CastToSH365GameInstance (Game|GetGameInstance)))
            (Variables|/Game/SH365GameInstance.SH365GameInstance_C|SetINS_PWLastLevel _assh365game_instance_4 true)
            (elif (Utilities|Enum|Equal(Enum) (Utilities|String|ToString(Text) (Variables|/Game/SH365GameInstance.SH365GameInstance_C|GetINS_PWStr _assh365game_instance)) (Variables|/Game/SH365GameInstance.SH365GameInstance_C|GetLevel2PW _assh365game_instance))
              (goto _label_6)
              (elif (Utilities|Enum|Equal(Enum) (Utilities|String|ToString(Text) (Variables|/Game/SH365GameInstance.SH365GameInstance_C|GetINS_PWStr _assh365game_instance)) (Variables|/Game/SH365GameInstance.SH365GameInstance_C|GetLevel1PW _assh365game_instance))
                (goto _label_6)
                (elif (Utilities|Enum|Equal(Enum) (Utilities|String|ToString(Text) (Variables|/Game/SH365GameInstance.SH365GameInstance_C|GetINS_PWStr _assh365game_instance)) (Variables|/Game/SH365GameInstance.SH365GameInstance_C|GetLevel1PW _assh365game_instance))
                  (goto _label_6))))))
        (:6
          (bind _assh365game_instance_5 (Utilities|Casting|CastToSH365GameInstance (Game|GetGameInstance)))
          (Variables|/Game/SH365GameInstance.SH365GameInstance_C|SetWeakFlag _assh365game_instance true))))))

(fn CheckWeakPW
  (bind _assh365game_instance (Utilities|Casting|CastToSH365GameInstance (Game|GetGameInstance)))
  (bind _outrownames (DataTable|GetDataTableRowNames "/Game/Level/1_Login/CSV/DT_PW.DT_PW"))
  (for _array_element _outrownames
    (bind _returnvalue (Utilities|GetDataTableRow "/Game/Level/1_Login/CSV/DT_PW.DT_PW" _array_element)
      (:then
        (if (Utilities|Enum|Equal(Enum) (Utilities|Struct|BreakST_PW _returnvalue) (Utilities|String|ToString(Text) (Variables|/Game/SH365GameInstance.SH365GameInstance_C|GetINS_PWStr _assh365game_instance)))
          (Development|PrintString "PWWEEEEEEEEEEEEEEEEEEEEEEK!")
          (Variables|/Game/SH365GameInstance.SH365GameInstance_C|SetINS_500-worst-password _assh365game_instance true))))))

(fn CheckSQLi
  (bind _assh365game_instance (Utilities|Casting|CastToSH365GameInstance (Game|GetGameInstance)))
  (bind _outrownames (DataTable|GetDataTableRowNames "/Game/Level/1_Login/CSV/DT_SQLi.DT_SQLi"))
  (for _array_element _outrownames
    (bind _returnvalue (Utilities|GetDataTableRow "/Game/Level/1_Login/CSV/DT_SQLi.DT_SQLi" _array_element)
      (:then
        (if (Utilities|Enum|Equal(Enum) (Utilities|Struct|BreakST_SQLi _returnvalue) (Utilities|String|ToString(Text) (Variables|/Game/SH365GameInstance.SH365GameInstance_C|GetINS_PWStr _assh365game_instance)))
          (Development|PrintString "SQLINJECTION!SQLINJECTION!SQLINJECTION!SQLINJECTION!SQLINJECTION!SQLINJECTION!SQLINJECTION!")
          (Variables|/Game/SH365GameInstance.SH365GameInstance_C|SetINS_SQLi _assh365game_instance true))))))

(fn ZxcvbnReason
  (bind _returnvalue (Actor|GetActorOfClass "/Script/SecHack.CheckPW"))
  (bind _output_get (LocalVariables|Setbruteforce (Utilities|String|FindSubstring (Variables|/Script/SecHack.CheckPW|GetzxcvbnResult2 _returnvalue) "Type: Bruteforce" true true)))
  (bind _output_get_2 (LocalVariables|Setdictionary (Utilities|String|FindSubstring (Variables|/Script/SecHack.CheckPW|GetzxcvbnResult2 _returnvalue) "Type: Dictionary" true true)))
  (bind _output_get_3 (LocalVariables|Setdictleeet (Utilities|String|FindSubstring (Variables|/Script/SecHack.CheckPW|GetzxcvbnResult2 _returnvalue) "Type: Dict+Leet" true true)))
  (bind _output_get_4 (LocalVariables|Setuserwords (Utilities|String|FindSubstring (Variables|/Script/SecHack.CheckPW|GetzxcvbnResult2 _returnvalue) "Type: User Words" true true)))
  (bind _output_get_5 (LocalVariables|Setuserleet (Utilities|String|FindSubstring (Variables|/Script/SecHack.CheckPW|GetzxcvbnResult2 _returnvalue) "Type: User+Leet" true true)))
  (bind _output_get_6 (LocalVariables|Setrepeated (Utilities|String|FindSubstring (Variables|/Script/SecHack.CheckPW|GetzxcvbnResult2 _returnvalue) "Type: Repeated" true true)))
  (bind _output_get_7 (LocalVariables|Setsequence (Utilities|String|FindSubstring (Variables|/Script/SecHack.CheckPW|GetzxcvbnResult2 _returnvalue) "Type: Sequence" true true)))
  (bind _output_get_8 (LocalVariables|Setspetial (Utilities|String|FindSubstring (Variables|/Script/SecHack.CheckPW|GetzxcvbnResult2 _returnvalue) "Type: Spatial" true true)))
  (bind _output_get_9 (LocalVariables|Setdata (Utilities|String|FindSubstring (Variables|/Script/SecHack.CheckPW|GetzxcvbnResult2 _returnvalue) "Type: Date" true true)))
  (bind _output_get_10 (LocalVariables|Setyear (Utilities|String|FindSubstring (Variables|/Script/SecHack.CheckPW|GetzxcvbnResult2 _returnvalue) "Type: Year" true true)))
  (bind _output_get_11 (LocalVariables|Setextra-long (Utilities|String|FindSubstring (Variables|/Script/SecHack.CheckPW|GetzxcvbnResult2 _returnvalue) "Type: Extra-long" true true)))
  (for _array_element (Utilities|Array|MakeArray _output_get _output_get_2 _output_get_3 _output_get_4 _output_get_5 _output_get_6 _output_get_7 _output_get_8 _output_get_9 _output_get_10 _output_get_11 0)
    _))